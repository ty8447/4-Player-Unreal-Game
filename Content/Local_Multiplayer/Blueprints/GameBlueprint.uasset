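; Local multiplayer game Blueprint that spawns and assigns characters for up to four players.
; Spawn1 to Spawn4 each destroy the given controller's current pawn, spawn that slot's own character class at a hardcoded location, possess it and store it in P1 to P4.
; GetPlayerStartPoints caches the level's PlayerStarts, but the spawn events ignore them, and the random-start logic in GetRandomSpawn is left unused.
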(event Custom|Spawn1
  (params (Player%20Controller :type Player%20Controller%20Object%20Reference))
  (bind _returnvalue (Pawn|GetControlledPawn Player%20Controller))
  ;[1 1 1] Spawn Characters (Controllers not currently bound to characters)
  (Class|GameplayStatics|GetPlayerControllerID Player%20Controller)
  (Utilities|IsValid _returnvalue
    (:Is%20Valid
      (Actor|DestroyActor _returnvalue))
    (:Is%20Not%20Valid
      _))
  (bind _returnvalue_2 (Game|SpawnActorfromClass "/Game/Local_Multiplayer/Models/Model/Character/Characterms.Characterms_C" (Math|Transform|MakeTransform "30.000000,-900.000000,112.000000" "0, 0, 0" "1,1,1") "AlwaysSpawn" 0 0))
  (Pawn|Possess Player%20Controller _returnvalue_2)
  (Variables|Default|SetP1 (Utilities|Array|MakeArray _returnvalue_2)))

(event Custom|Spawn2
  (params (Player%20Controller :type Player%20Controller%20Object%20Reference))
  (bind _returnvalue (Pawn|GetControlledPawn Player%20Controller))
  ;[1 1 1] Spawn Characters (Controllers not currently bound to characters)
  (Class|GameplayStatics|GetPlayerControllerID Player%20Controller)
  (Utilities|IsValid _returnvalue
    (:Is%20Valid
      (Actor|DestroyActor _returnvalue))
    (:Is%20Not%20Valid
      _))
  (bind _returnvalue_2 (Game|SpawnActorfromClass "/Game/Local_Multiplayer/Models/Model/Character/Characterms2.Characterms2_C" (Math|Transform|MakeTransform "-950.000000,790.000000,112.000000" "0, 0, 0" "1,1,1") "AlwaysSpawn" 0 0))
  (Pawn|Possess Player%20Controller _returnvalue_2)
  (Variables|Default|SetP2 (Utilities|Array|MakeArray _returnvalue_2)))

(event Custom|Spawn3
  (params (Player%20Controller :type Player%20Controller%20Object%20Reference))
  (bind _returnvalue (Pawn|GetControlledPawn Player%20Controller))
  ;[1 1 1] Spawn Characters (Controllers not currently bound to characters)
  (Class|GameplayStatics|GetPlayerControllerID Player%20Controller)
  (Utilities|IsValid _returnvalue
    (:Is%20Valid
      (Actor|DestroyActor _returnvalue))
    (:Is%20Not%20Valid
      _))
  (bind _returnvalue_2 (Game|SpawnActorfromClass "/Game/Local_Multiplayer/Models/Model/Character/Characterms3.Characterms3_C" (Math|Transform|MakeTransform "317.000000,787.000000,112.000000" "0, 0, 0" "1,1,1") "AlwaysSpawn" 0 0))
  (Pawn|Possess Player%20Controller _returnvalue_2)
  (Variables|Default|SetP3 (Utilities|Array|MakeArray _returnvalue_2)))

(event Custom|Spawn4
  (params (PlayerController :type Player%20Controller%20Object%20Reference))
  (bind _returnvalue (Pawn|GetControlledPawn PlayerController))
  ;[1 1 1] Spawn Characters (Controllers not currently bound to characters)
  (Class|GameplayStatics|GetPlayerControllerID PlayerController)
  (Utilities|IsValid _returnvalue
    (:Is%20Valid
      (Actor|DestroyActor _returnvalue))
    (:Is%20Not%20Valid
      _))
  (bind _returnvalue_2 (Game|SpawnActorfromClass "/Game/Local_Multiplayer/Models/Model/Character/Characterms4.Characterms4_C" (Math|Transform|MakeTransform "580.000000,-830.000000,112.000000" "0, 0, 0" "1,1,1") "AlwaysSpawn" 0 0))
  (Pawn|Possess PlayerController _returnvalue_2)
  (Variables|Default|SetP4 (Utilities|Array|MakeArray _returnvalue_2)))

(fn ConstructionScript)

(fn GetPlayerStartPoints
  (bind _outactors (Actor|GetAllActorsOfClass "/Script/Engine.PlayerStart"))
  (Variables|Default|SetPlayerStartArray _outactors))
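; Local multiplayer manager that creates the local players and swaps them between placeholder IntPawns and playable characters.
; BeginPlay matches PlayerStart tags to player indices, creating each player and spawning an IntPawn there.
; Spawn1–4 assign a controller ID, replace the controlled pawn with that slot's character class at a hardcoded location, and possess it.
; DespawnCharacter reverts to an IntPawn via GetRandomSpawn; SpawnPlayers, a single-class tag-based alternative, is uncalled here.
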(event Custom|Spawn1
  (params (Player%20Controller :type Player%20Controller%20Object%20Reference))
  (bind _returnvalue (Pawn|GetControlledPawn Player%20Controller))
  ;[1 1 1] Spawn Characters Events
  (Class|GameplayStatics|SetPlayerControllerID Player%20Controller)
  (Utilities|IsValid _returnvalue
    (:Is%20Valid
      (Actor|DestroyActor _returnvalue))
    (:Is%20Not%20Valid
      _))
  (bind _returnvalue_2 (Game|SpawnActorfromClass "/Game/Local_Multiplayer/Models/Model/Character/Characterms.Characterms_C" (Math|Transform|MakeTransform "-590.000000,-170.000000,662.062622" "0,180.000000, 0" "1,1,1") "AlwaysSpawn" 0 0))
  (Pawn|Possess Player%20Controller _returnvalue_2))

(event Custom|Spawn2
  (params (Player%20Controller :type Player%20Controller%20Object%20Reference))
  (bind _returnvalue (Pawn|GetControlledPawn Player%20Controller))
  ;[1 1 1] Spawn Characters Events
  (Class|GameplayStatics|SetPlayerControllerID Player%20Controller 1)
  (Utilities|IsValid _returnvalue
    (:Is%20Valid
      (Actor|DestroyActor _returnvalue))
    (:Is%20Not%20Valid
      _))
  (bind _returnvalue_2 (Game|SpawnActorfromClass "/Game/Local_Multiplayer/Models/Model/Character/Characterms2.Characterms2_C" (Math|Transform|MakeTransform "-590.000000,565.000000,662.062622" "0,180.000000, 0" "1,1,1") "AlwaysSpawn" 0 0))
  (Pawn|Possess Player%20Controller _returnvalue_2))

(event Custom|Spawn3
  (params (Player%20Controller :type Player%20Controller%20Object%20Reference))
  (bind _returnvalue (Pawn|GetControlledPawn Player%20Controller))
  ;[1 1 1] Spawn Characters Events
  (Class|GameplayStatics|SetPlayerControllerID Player%20Controller 2)
  (Utilities|IsValid _returnvalue
    (:Is%20Valid
      (Actor|DestroyActor _returnvalue))
    (:Is%20Not%20Valid
      _))
  (bind _returnvalue_2 (Game|SpawnActorfromClass "/Game/Local_Multiplayer/Models/Model/Character/Characterms3.Characterms3_C" (Math|Transform|MakeTransform "-705.000000,-170.000000,112.062599" "0,180.000000, 0" "1,1,1") "AlwaysSpawn" 0 0))
  (Pawn|Possess Player%20Controller _returnvalue_2))

(event Custom|Spawn4
  (params (PlayerController :type Player%20Controller%20Object%20Reference))
  (bind _returnvalue (Pawn|GetControlledPawn PlayerController))
  ;[1 1 1] Spawn Characters Events
  (Class|GameplayStatics|SetPlayerControllerID PlayerController 3)
  (Utilities|IsValid _returnvalue
    (:Is%20Valid
      (Actor|DestroyActor _returnvalue))
    (:Is%20Not%20Valid
      _))
  (bind _returnvalue_2 (Game|SpawnActorfromClass "/Game/Local_Multiplayer/Models/Model/Character/Characterms4.Characterms4_C" (Math|Transform|MakeTransform "-665.000000,530.000000,112.062599" "0,180.000000, 0" "1,1,1") "AlwaysSpawn" 0 0))
  (Pawn|Possess PlayerController _returnvalue_2))

(event Custom|DespawnCharacter
  (params (PlayerController :type Player%20Controller%20Object%20Reference))
  (bind _returnvalue (Pawn|GetControlledPawn PlayerController))
  ;[1 1 1] Despawn Characters
  (Utilities|IsValid _returnvalue
    (:Is%20Valid
      (Actor|DestroyActor _returnvalue)
      (bind _returnvalue_2 (Game|SpawnActorfromClass "/Game/Local_Multiplayer/Maps/Testing/intPawn.intPawn_C" (Utilities|GetRandomSpawn) "Undefined" 0 0))
      (Pawn|Possess PlayerController _returnvalue_2))))

(event EventBeginPlay
  ;[1 1 1] Spawn blank Characters
  (CallFunction|GetPlayerStartPoints)
  (for _index (range 0 (- (Variables|Default|GetMaxPlayerCount) 1))
    (Variables|Default|SetIndex _index)
    (for _array_element (Variables|Default|GetPlayerStartArray)
      (if (Utilities|Name|Equal(Name) (Variables|/Script/Engine.PlayerStart|GetPlayerStartTag _array_element) (Utilities|String|StringToName (Utilities|String|ToString(Integer) (Variables|Default|GetIndex))))
        (Class|GameplayStatics|CreatePlayer (Variables|Default|GetIndex))
        (Game|SpawnActorfromClass "/Game/Local_Multiplayer/Maps/Testing/intPawn.intPawn_C" (Transformation|GetActorTransform _array_element) "Undefined" 0 0)))))

(fn ConstructionScript)

(fn SpawnPlayers
  ;[1 1 1] One Spawn System
  (for _index (range 0 (- (Variables|Default|GetMaxPlayerCount) 1))
    (Variables|Default|SetIndex _index)
    (for _array_element (Variables|Default|GetPlayerStartArray)
      (if (Utilities|Name|Equal(Name) (Variables|/Script/Engine.PlayerStart|GetPlayerStartTag _array_element) (Utilities|String|StringToName (Utilities|String|ToString(Integer) (Variables|Default|GetIndex))))
        (Class|GameplayStatics|CreatePlayer (Variables|Default|GetIndex))
        (bind _returnvalue (Game|SpawnActorfromClass "/Game/Local_Multiplayer/Models/Model/Character/Characterms.Characterms_C" (Transformation|GetActorTransform _array_element) "DontSpawnIfColliding" 0 0))
        (Pawn|Possess (Game|GetPlayerController (Variables|Default|GetIndex)) _returnvalue)))))

(fn GetPlayerStartPoints
  (bind _outactors (Actor|GetAllActorsOfClass "/Script/Engine.PlayerStart"))
  (Variables|Default|SetPlayerStartArray _outactors))